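; Third-person shooter player Blueprint that handles sniper scope zoom and weapon mesh switching.
; It creates the sniper scope widget at BeginPlay, then holding Zoom shows it, narrows the TPS camera FOV and hides the crosshair, with release reversing all three.
; ChangeGun toggles visibility between the grenade gun and sniper meshes from a single IsGrenade flag.
; The crosshair widget is only referenced here, guarded by validity checks, and is not created in this graph.
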(event `InputAction|Zoom`
  (params (Key :type "Key Structure"))
  (bind _sniperui (`self.SniperUI`))
  (bind _tpscamcomp (`self.tpsCamComp`))
  (bind _crosshairui (`self.crosshairUI`))
  (:`Pressed`
    (`UserWidget.AddToViewport` _sniperui 0)
    (`CameraComponent.SetFieldOfView` _tpscamcomp 20.5)
    (`/Engine/EditorBlueprintResources/StandardMacros.IsValid` _crosshairui
      (:`Is Valid`
        (`Widget.RemoveFromParent` _crosshairui))))
  (:`Released`
    (`Widget.RemoveFromParent` _sniperui)
    (`CameraComponent.SetFieldOfView` _tpscamcomp 90.0)
    (`/Engine/EditorBlueprintResources/StandardMacros.IsValid` _crosshairui
      (:`Is Valid`
        (`UserWidget.AddToViewport` _crosshairui 0)))))

(event `self.ReceiveBeginPlay`
  ;[1 1 1] SniperScope 위젯 인스턴스 만들기
  (bind _returnvalue (`|CreateWidget` "/Game/Blueprints/WBP_SniperUI.WBP_SniperUI_C"))
  (set `self.SniperUI` _returnvalue))

(fn `ChangeGun`
  (params (`IsGrenade?` :type Boolean))
  (`SceneComponent.SetVisibility` (`self.gunMeshComp`) `IsGrenade?` false)
  (`SceneComponent.SetVisibility` (`self.sniperGunComp`) (not `IsGrenade?`) false))

(fn `UserConstructionScript`)